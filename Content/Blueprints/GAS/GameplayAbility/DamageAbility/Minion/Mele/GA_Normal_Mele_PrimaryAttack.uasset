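; Gameplay ability for a minion's normal melee primary attack, dealing damage to an enemy caught in the character's melee collision boundary.
; Activation plays the attack montage, binds to the boundary's begin-overlap event, and ends the ability when the montage completes, is interrupted or is cancelled.
; Overlapped characters with a different team tag receive an effect spec built from the damage-type map, then the boundary ignores all channels to stop further hits.
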(event Custom|OnComponentBeginOverlap_Event
  (params (OverlappedComponent :type Primitive%20Component%20Object%20Reference) (OtherActor :type Actor%20Object%20Reference) (OtherComp :type Primitive%20Component%20Object%20Reference) (OtherBodyIndex :type Integer) (bFromSweep :type Boolean) (SweepResult :type Hit%20Result%20Structure%20%28by%20ref%29))
  (bind _returnvalue (Ability|GetAvatarActorfromActorInfo))
  (Variables|Default|SetOverlappedActor OtherActor)
  (if (!= OtherActor _returnvalue)
    (bind _asbase_character (Utilities|Casting|CastToBaseCharacter _returnvalue)) ; OwnerActor
    (bind _asbase_character_2 (Utilities|Casting|CastToBaseCharacter (Variables|Default|GetOverlappedActor))) ; Overlapped Actor
    (bind _returnvalue_2 (Class|BaseCharacter|GetTeamTag _asbase_character))
    (bind _returnvalue_3 (Class|BaseCharacter|GetTeamTag _asbase_character_2))
    (if (!= _returnvalue_3 _returnvalue_2)
      (bind _returnvalue_4 (Class|MyBlueprintFunctionLibrary|MakeEffectSpecHandlewithDamageTypeMap (Variables|Default|GetEffectClass) (Ability|GetAbilitySystemComponentfromActorInfo) self (Variables|Default|GetEffectTypeMap)))
      (GameplayEffects|ApplyGameplayEffectSpecToSelf (Ability|GetAbilitySystemComponent OtherActor) _returnvalue_4)
      (Collision|SetCollisionResponsetoAllChannels (Class|BaseCharacter|GetMeleCollisionBoundary (Variables|Default|GetAs%20Base%20Character)) "ECR_Ignore"))))

(event Ability|EventOnEndAbility
  (params (bWasCancelled :type Boolean))
  (|CallParentFunction bWasCancelled) ; This node is disabled and will not be called.\nDrag off pins to build functionality.
)

(event Ability|EventActivateAbility
  (|PlayMontageandWaitProxy "None" (Variables|Default|GetAbilityAnimMontage) 1.0 "None" true 1.0 0.0 false
    (:then
      (bind _asbase_character (Utilities|Casting|CastToBaseCharacter (Ability|GetAvatarActorfromActorInfo)))
      (Variables|Default|SetAs%20Base%20Character _asbase_character)
      (Collision|AssignOnComponentBeginOverlap (Class|BaseCharacter|GetMeleCollisionBoundary _asbase_character) (delegate Custom|OnComponentBeginOverlap_Event)))
    (:OnCompleted
      (Ability|EndAbility :!label _label))
    (:OnInterrupted
      (goto _label))
    (:OnCancelled
      (goto _label))))