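; Gameplay ability for the Super melee minion's primary attack, dealing damage through GAS effects.
; On activation it plays the attack montage, binds to the avatar's melee collision overlap, and ends when the montage completes, blends out or is interrupted or cancelled.
; Each overlapped actor other than the avatar receives an effect spec built from the effect class and type map.
; The graph never explicitly unbinds the overlap delegate.
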(event Custom|OnComponentBeginOverlap_Event
  (params (OverlappedComponent :type Primitive%20Component%20Object%20Reference) (OtherActor :type Actor%20Object%20Reference) (OtherComp :type Primitive%20Component%20Object%20Reference) (OtherBodyIndex :type Integer) (bFromSweep :type Boolean) (SweepResult :type Hit%20Result%20Structure%20%28by%20ref%29))
  (if (!= OtherActor (Ability|GetAvatarActorfromActorInfo))
    (bind _returnvalue (Class|MyBlueprintFunctionLibrary|MakeEffectSpecHandlewithDamageTypeMap (Variables|Default|GetEffectClass) (Ability|GetAbilitySystemComponentfromActorInfo) self (Variables|Default|GetEffectTypeMap)))
    (GameplayEffects|ApplyGameplayEffectSpecToSelf (Ability|GetAbilitySystemComponent OtherActor) _returnvalue)))

(event Ability|EventOnEndAbility
  (params (bWasCancelled :type Boolean))
  (|CallParentFunction bWasCancelled) ; This node is disabled and will not be called.\nDrag off pins to build functionality.
)

(event Ability|EventActivateAbility
  (|PlayMontageandWaitProxy "None" (Variables|Default|GetAbilityAnimMontage) 1.0 "None" true 1.0 0.0 false
    (:then
      (bind _asbase_character (Utilities|Casting|CastToBaseCharacter (Ability|GetAvatarActorfromActorInfo)))
      (Collision|AssignOnComponentBeginOverlap (Class|BaseCharacter|GetMeleCollisionBoundary _asbase_character) (delegate Custom|OnComponentBeginOverlap_Event)))
    (:OnCompleted
      (Ability|EndAbility :!label _label))
    (:OnBlendOut
      (goto _label))
    (:OnInterrupted
      (goto _label))
    (:OnCancelled
      (goto _label))))