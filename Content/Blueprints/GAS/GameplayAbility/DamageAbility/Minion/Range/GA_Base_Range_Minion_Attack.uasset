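; Gameplay ability for a ranged minion's basic attack, firing a projectile at the avatar's current target.
; Activation plays the attack montage and starts attack motion warping toward the target's location.
; A one-shot gameplay event matching the ability tag spawns a moving projectile from the front muzzle socket, aimed at the target's location at that moment.
; The ability ends when the montage finishes or is interrupted, or when the target is invalid.
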(event Ability|EventActivateAbility
  (|PlayMontageandWaitProxy "None" (Variables|Default|GetAbilityAnimMontage) 1.0 "None" true 1.0 0.0 false
    (:then
      (bind _asbase_character (Utilities|Casting|CastToBaseCharacter (Ability|GetAvatarActorfromActorInfo)))
      (bind _output_get (Variables|Default|SetOwnerTypeBaseChar _asbase_character))
      (bind _currenttargetactor (Variables|/Script/Project_MOBA.BaseCharacter|GetCurrentTargetActor _output_get)
        (:then
          (bind _asbp_base_minion (Utilities|Casting|CastToBP_BaseMinion _output_get))
          (Default|StartAttackWarpMotion _asbp_base_minion "AttackWarpMotion" (Math|Transform|MakeTransform (Transformation|GetActorLocation _currenttargetactor) "0, 0, 0" "1.000000,1.000000,1.000000"))
          (Ability|Tasks|WaitGameplayEvent (Variables|Default|GetAbilityTag) 0 true
            (:EventReceived
              (bind _currenttargetactor_2 (Variables|/Script/Project_MOBA.BaseCharacter|GetCurrentTargetActor (Variables|Default|GetOwnerTypeBaseChar))
                (:then
                  (Class|ProjectileEffectAbility|SpawnProjectileatSocket (Transformation|GetActorLocation _currenttargetactor_2) false "Muzzle_Front" "1.000000,1.000000,1.000000" true 5e+03))
                (:else
                  (Ability|EndAbility))))))
        (:else
          (Ability|EndAbility))))
    (:OnCompleted
      (Ability|EndAbility :!label _label))
    (:OnBlendOut
      (goto _label))
    (:OnInterrupted
      (goto _label))
    (:OnCancelled
      (goto _label))))

(event Ability|EventOnEndAbility
  (params (bWasCancelled :type Boolean))
  (|CallParentFunction bWasCancelled) ; This node is disabled and will not be called.\nDrag off pins to build functionality.
)