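; Gameplay ability for a normal ranged minion's primary attack, firing a projectile at the minion's current target.
; On activation it plays the attack montage and starts the minion's attack motion warp toward the target's location.
; A gameplay event matching the ability tag triggers a single projectile from the front muzzle socket at the target's position at that moment.
; The ability ends when the montage completes, blends out, is interrupted or is cancelled.
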(event Ability|EventActivateAbility
  (|PlayMontageandWaitProxy "None" (Variables|Default|GetAbilityAnimMontage) 1.0 "None" true 1.0 0.0 false
    (:then
      (bind _asbp_base_minion (Utilities|Casting|CastToBP_BaseMinion (Ability|GetAvatarActorfromActorInfo))
        (:then
          (Variables|Default|SetAs%20BP%20Base%20Minion _asbp_base_minion))
        (:CastFailed
          _))
      (Default|StartAttackWarpMotion _asbp_base_minion "AttackWarpMotion" (Math|Transform|MakeTransform (Transformation|GetActorLocation (Variables|/Game/Blueprints/Characters/Minions/BP_BaseMinion.BP_BaseMinion_C|GetTargetActor _asbp_base_minion)) "0, 0, 0" "1.000000,1.000000,1.000000"))
      (Ability|Tasks|WaitGameplayEvent (Variables|Default|GetAbilityTag) 0 true
        (:EventReceived
          (Class|ProjectileEffectAbility|SpawnProjectileatSocket (Transformation|GetActorLocation (Variables|/Game/Blueprints/Characters/Minions/BP_BaseMinion.BP_BaseMinion_C|GetTargetActor (Variables|Default|GetAs%20BP%20Base%20Minion))) false "Muzzle_Front" "1.000000,1.000000,1.000000" true 5e+03))))
    (:OnCompleted
      (Ability|EndAbility :!label _label))
    (:OnBlendOut
      (goto _label))
    (:OnInterrupted
      (goto _label))
    (:OnCancelled
      (goto _label))))

(event Ability|EventOnEndAbility
  (params (bWasCancelled :type Boolean))
  (|CallParentFunction bWasCancelled) ; This node is disabled and will not be called.\nDrag off pins to build functionality.
)