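; Base projectile Gameplay Ability that fires a projectile at a targeted hit location, timed to an attack montage.
; A target-data task supplies the hit result, then the montage plays while a player-character avatar motion-warps toward that location.
; The FireBall gameplay event, hardcoded here, triggers the projectile spawn from a socket toward the target.
; The ability ends when the montage completes, is interrupted or is cancelled.
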(event Ability|EventActivateAbility
  (bind _hitresult (|AbilityTaskTargetHitResult)
    (:TargetDataHitResultDelegate
      (|PlayMontageandWaitProxy "None" (Variables|Default|GetMontage%20to%20Play) 1.0 "None" true 1.0 0.0 false
        (:then
          (bind _asbp_player_character (Utilities|Casting|CastToBP_PlayerCharacter (Ability|GetAvatarActorfromActorInfo))
            (:then
              (Default|StartAttackWarpMotion _asbp_player_character (Variables|Default|GetWarp%20Motion%20Name) (Math|Conversions|ToTransform(Vector) (.Location (Collision|BreakHitResult (Ability|TargetData|GetHitResultfromTargetData _hitresult))))))
            (:CastFailed
              _))
          (Ability|Tasks|WaitGameplayEvent "(TagName=\"Ability.Projectile.FireBall\")" 0
            (:EventReceived
              (Class|ProjectileAbility|SpawnProjectile (.Location (Collision|BreakHitResult (Ability|TargetData|GetHitResultfromTargetData _hitresult))) (Variables|Default|GetSpawn%20Socket%20Location) "0.700000,0.700000,0.700000"))))
        (:OnCompleted
          (Ability|EndAbility :!label _label))
        (:OnInterrupted
          (goto _label))
        (:OnCancelled
          (goto _label))))))

(event Ability|EventOnEndAbility
  (params (bWasCancelled :type Boolean)))