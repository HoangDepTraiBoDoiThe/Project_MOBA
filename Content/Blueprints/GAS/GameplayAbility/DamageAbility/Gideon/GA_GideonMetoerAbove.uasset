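; Gideon's gameplay ability that launches a meteor projectile from above the caster toward a selected target location.
; On BeginSpawnProjectile it calls SpawnProjectileAtSelectedLocation with a spawn point high over the avatar, passing the target, scale and speed for a moving projectile.
; Its own activate and end events are disabled stubs, so the rest of the ability flow is left to the parent class.
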(event Ability|EventActivateAbility
  (|CallParentFunction) ; This node is disabled and will not be called.\nDrag off pins to build functionality.
)

(event Ability|EventOnEndAbility
  (params (bWasCancelled :type Boolean))
  (|CallParentFunction bWasCancelled) ; This node is disabled and will not be called.\nDrag off pins to build functionality.
)

(event EventBeginSpawnProjectile
  (bind _returnvalue (Ability|GetAvatarActorfromActorInfo))
  (bind _returnvalue_2 (Transformation|GetActorLocation _returnvalue))
  (Class|ProjectileEffectAbility|SpawnProjectileatSelectedLocation (Variables|Default|GetTargetLocation) false (Math|Vector|MakeVector (.x _returnvalue_2) (.y _returnvalue_2) (+ 7e+02 (.z _returnvalue_2))) (Variables|Default|GetProjectile%20Scale) true (Variables|Default|GetProjectileSpeed)))