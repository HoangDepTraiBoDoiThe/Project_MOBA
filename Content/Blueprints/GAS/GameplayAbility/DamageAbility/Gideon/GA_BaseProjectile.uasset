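; GA_BaseProjectile is a base gameplay ability for targeted projectile attacks, with an empty BeginSpawnProjectile hook for the actual spawn.
; On activation it commits, then stores the target location and hit actor from a hit-result targeting task.
; It plays the ability montage, starts motion warping on the player character toward the target, and calls the hook when the ability's gameplay event arrives.
; The ability ends when the montage completes, is interrupted or is cancelled.
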(event Custom|AbilityActivating)

(event Ability|EventActivateAbility
  (Ability|CommitAbility)
  (bind _hitresult (|AbilityTaskTargetHitResult)
    (:TargetDataHitResultDelegate
      (Variables|GABasePrjectile|SetTargetLocation (.Location (Collision|BreakHitResult (Ability|TargetData|GetHitResultfromTargetData _hitresult))))
      (Variables|Default|SetHit%20Actor (.HitActor (Collision|BreakHitResult (Ability|TargetData|GetHitResultfromTargetData _hitresult))))
      (|PlayMontageandWaitProxy "None" (Variables|Default|GetAbilityAnimMontage) 1.0 "None" true 1.0 0.0 false
        (:then
          (bind _asbp_player_character (Utilities|Casting|CastToBP_PlayerCharacter (Ability|GetAvatarActorfromActorInfo))
            (:then
              (Default|StartAttackWarpMotion _asbp_player_character (Variables|GABasePrjectile|GetWarp%20Motion%20Name) (Math|Conversions|ToTransform(Vector) (Variables|GABasePrjectile|GetTargetLocation))))
            (:CastFailed
              _))
          (Ability|Tasks|WaitGameplayEvent (Variables|Default|GetAbilityTag) 0
            (:EventReceived
              (CallFunction|BeginSpawnProjectile))))
        (:OnCompleted
          (Ability|EndAbility :!label _label))
        (:OnInterrupted
          (goto _label))
        (:OnCancelled
          (goto _label))))))

(fn BeginSpawnProjectile)