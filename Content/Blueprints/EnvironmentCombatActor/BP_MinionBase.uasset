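; BP_MinionBase is an environment combat actor that spawns minions in timed waves.
; On BeginPlay it waits an initial delay, then gets the wave's class list from GetNextWaveToResponse.
; A delay-driven loop passes classes to SpawnAMinion at a set rate, then waits before fetching the next wave.
; The Counter index has no reset in this graph and its <= check runs past the list's end; an alternative ForEach spawn path is unconnected.
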(event EventBeginPlay
  (Utilities|FlowControl|Delay (Variables|Default|GetDelayFirstSpawn))
  (bind _returnvalue (Class|MinionBase|GetNextWavetoResponse :!label _label))
  (bind _output_get (Variables|Default|SetNextWaveClasses _returnvalue))
  (Variables|Default|SetTotalMinionCount (Utilities|Array|Length _output_get))
  (if (<= (Variables|Default|GetCounter) (Variables|Default|GetTotalMinionCount)) :!label _label_2
    (Class|MinionBase|SpawnAMinion (Utilities|Array|Get(acopy) (Variables|Default|GetNextWaveClasses) (Variables|Default|GetCounter)))
    (Math|Integer|IncrementInt (Variables|Default|GetCounter)
      (:%20%20
        (Utilities|FlowControl|Delay (Variables|Default|GetRate))
        (goto _label_2)))
    (else
      (Utilities|FlowControl|Delay (Variables|Default|GetWaveSpawnRate))
      (goto _label))))

(event Collision|EventActorBeginOverlap
  (params (OtherActor :type Actor%20Object%20Reference)))

(event EventTick
  (params (DeltaSeconds :type Float%20%28single-precision%29)))

(fn ConstructionScript)